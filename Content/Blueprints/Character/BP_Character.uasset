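; Top-down player character Blueprint with a zoomable spring-arm camera, walk, sprint and aim states, and rifle fire montages.
; Mouse wheel input steps the boom length between height limits, either instantly or smoothly through a looping timer.
; Walk, sprint and aim inputs set flags and call ChageMovementState, while a timer drains and regenerates sprint stamina, stored in SprintDirection.
; Left click plays a hip or ironsights montage, and a separate function plays camera shake.
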(event `InputAxis|MouseWheel`
  (params (AxisValue :type "Float (single-precision)"))
  (if (`self.SlideWithSmooth`)
    (`self.CameraSlideSmooth` AxisValue)
    (else
      (`self.CameraSlide` AxisValue))))

(event `InputAction|MovementModeChangeWalk`
  (params (Key :type "Key Structure"))
  (:`Pressed`
    (set `self.WalkEnabled` true)
    (`self.ChageMovementState` :!label _label))
  (:`Released`
    (set `self.WalkEnabled` false)
    (goto _label)))

(event `InputAction|MovementModeChangeSprint`
  (params (Key :type "Key Structure"))
  (:`Pressed`
    (set `self.SprintRunEnabled` true)
    (`|ExecutionSequence`
      (:`then_0`
        (bind _returnvalue (`KismetSystemLibrary.K2_SetTimerDelegate` (delegate `StaminaTick`) 1.0 true))
        (set `self.StaminaTimer` _returnvalue)
        (`self.StaminaTick`))
      (:`then_1`
        (goto _label))))
  (:`Released`
    (set `self.SprintRunEnabled` false)
    (goto _label)))

(event `StaminaTick`
  (if (and (`self.SprintRunEnabled`) (> (`self.SprintDirection`) 0.0))
    (bind _output_get (set `self.SprintDirection` (- (`self.SprintDirection`) 10.0)))
    (if (<= _output_get 0.0)
      (set `self.SprintDirection` 0.0)
      (set `self.SprintRunEnabled` false)
      (`self.ChageMovementState`))
    (else
      (set `self.SprintRunEnabled` false)
      (`self.ChageMovementState`)
      (bind _output_get_2 (set `self.SprintDirection` (+ (`self.SprintDirection`) 5.0)))
      (if (>= _output_get_2 100.0)
        (`KismetSystemLibrary.K2_ClearAndInvalidateTimerHandle` (`self.StaminaTimer`))
        (set `self.SprintDirection` 100.0)))))

(event `Key|RightMouseButton`
  (params (Key :type "Key Structure"))
  (:`Pressed`
    (set `self.AimEnabled` true)
    (goto _label))
  (:`Released`
    (set `self.AimEnabled` false)
    (goto _label)))

(event `Key|LeftMouseButton`
  (params (Key :type "Key Structure"))
  (bind _mesh (`self.Mesh`))
  (:`Pressed`
    (if (`self.AimEnabled`)
      (`|PlayMontage` _mesh "/Game/Blueprints/Character/Mannequin/Animations/NewAnimation/NewFire_Rifle_Ironsights_Montage.NewFire_Rifle_Ironsights_Montage")
      (else
        (`|PlayMontage` _mesh "/Game/Blueprints/Character/Mannequin/Animations/NewAnimation/NewFire_Rifle_Hip_Montage.NewFire_Rifle_Hip_Montage")))))

(fn `CameraShakeEvent`
  (`GameplayStatics.PlayWorldCameraShake` "/Game/Blueprints/Game/BP_CameraShake.BP_CameraShake_C" (`SceneComponent.K2_GetComponentLocation` (`self.TopDownCameraComponent`)) 0.0 30.0))

(fn `CameraSlide`
  (params (Value :type "Float (double-precision)"))
  (bind _cameraboom (`self.CameraBoom`))
  (bind _heightcamerachangedistace (`self.HeightCameraChangeDistace`))
  (bind _targetarmlength (`SpringArmComponent.TargetArmLength` _cameraboom))
  (bind _returnvalue (- _targetarmlength _heightcamerachangedistace))
  (bind _returnvalue_2 (+ _targetarmlength _heightcamerachangedistace))
  (if (!= Value 0.0)
    (if (< Value 0.0)
      (if (>= (`self.HeightCameraMax`) _returnvalue_2)
        (set `SpringArmComponent.TargetArmLength` _returnvalue_2 _cameraboom))
      (elif (<= (`self.HieghtCameraMin`) _returnvalue)
        (set `SpringArmComponent.TargetArmLength` _returnvalue _cameraboom)))))

(fn `CameraSlideSmooth`
  (params (Value :type "Float (double-precision)"))
  (bind _heightcamerachangedistace (`self.HeightCameraChangeDistace`))
  (bind _targetarmlength (`SpringArmComponent.TargetArmLength` (`self.CameraBoom`)))
  (if (`self.SlideDone`)
    (if (!= Value 0.0)
      (if (< Value 0.0)
        (if (>= (`self.HeightCameraMax`) (+ _targetarmlength _heightcamerachangedistace))
          (set `self.SlideUp` true)
          (set `self.SlideDone` false :!label _label)
          (bind _returnvalue (`KismetSystemLibrary.K2_SetTimer` null "CameraSlideSmoothTick" (`self.TimerStep`) true))
          (set `self.SlideTimer` _returnvalue))
        (elif (<= (`self.HieghtCameraMin`) (- _targetarmlength _heightcamerachangedistace))
          (set `self.SlideUp` false)
          (goto _label))))))

(fn `CameraSlideSmoothTick`
  (locals (NewLocalVar_0 :type "TimerHandle Structure"))
  (bind _cameraboom (`self.CameraBoom`))
  (bind _heightchangeslidestepdistace (`self.HeightChangeSlideStepDistace`))
  (bind _targetarmlength (`SpringArmComponent.TargetArmLength` _cameraboom))
  (bind _output_get (set `self.CurrentSlideDistace` (+ (`self.CurrentSlideDistace`) _heightchangeslidestepdistace)))
  (set `SpringArmComponent.TargetArmLength` (select `bool` (`self.SlideUp`) :`false` (- _targetarmlength _heightchangeslidestepdistace) :`true` (+ _targetarmlength _heightchangeslidestepdistace)) _cameraboom)
  (if (>= _output_get (`self.HeightCameraChangeDistace`))
    (set `self.CurrentSlideDistace` 0.0)
    (set `self.SlideDone` true)
    (`KismetSystemLibrary.K2_ClearAndInvalidateTimerHandle` (`self.SlideTimer`))))

(fn `UserConstructionScript`
  (bind _cameraboom (`self.CameraBoom`))
  (set `SpringArmComponent.TargetArmLength` (`self.HieghtCameraMin`) _cameraboom)
  (`SceneComponent.K2_SetRelativeRotation` _cameraboom (`self.RotatorCamera`) false false)
  (set `SpringArmComponent.bEnableCameraLag` (`self.flow`) _cameraboom)
  (set `SpringArmComponent.CameraLagSpeed` (`self.CoefSmooth`) _cameraboom))